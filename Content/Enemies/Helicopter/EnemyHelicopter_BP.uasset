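; Enemy helicopter Actor that aims at and flies relative to a target and can break apart on hard impacts.
; On BeginPlay it passes its Target to separate aiming and flying components, which handle that behavior.
; Tick spins a static mesh about yaw by a fixed step per frame, independent of delta time.
; A helicopter mesh hit with a large enough normal impulse breaks the physics constraint; weaker hits print the impulse magnitude.
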(event `self.ReceiveBeginPlay`
  (bind _target (`self.Target`))
  (`EnemyAimComponent.Initialize` (`self.AimingComponent`) _target)
  (`EnemyFlyingComponent.Initialize` (`self.FlyingComponent`) _target))

(event `self.ReceiveTick`
  (params (DeltaSeconds :type "Float (single-precision)"))
  (`SceneComponent.K2_AddRelativeRotation` (`self.StaticMesh`) (`KismetMathLibrary.MakeRotator` 0.0 0.0 50.0) false false))

(event `self.HelicopterMesh.OnComponentHit`
  (params (HitComponent :type "PrimitiveComponent Object Reference") (OtherActor :type "Actor Object Reference") (OtherComp :type "PrimitiveComponent Object Reference") (NormalImpulse :type "Vector Structure") (Hit :type "HitResult Structure (by ref)"))
  (bind _returnvalue (`KismetMathLibrary.VSize` NormalImpulse))
  (if (> _returnvalue 150000.0)
    (`PhysicsConstraintComponent.BreakConstraint` (`self.PhysicsConstraint`))
    (else
      (`KismetSystemLibrary.PrintString` (`KismetStringLibrary.Conv_DoubleToString` _returnvalue)))))

(fn `UserConstructionScript`)