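; Punch-bag building actor on a physics constraint that absorbs heavy impacts until it breaks apart.
; Hit events on MovableMesh above an impulse threshold play an explosion sound, spawn debris effects and increment a counter.
; At the count limit, it hides the mesh and constraint, spawns smoke and adds a destructible-mesh component at runtime.
; Tick re-arms hit detection through a time check, but HitTimer never records the hit time.
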(event `self.ReceiveTick`
  (params (DeltaSeconds :type "Float (single-precision)"))
  (if (>= (- (`GameplayStatics.GetTimeSeconds`) (`self.HitTimer`)) 1.0)
    (set `self.HitTimer` 0.0)
    (set `self.CanHit` true)))

(event `self.MovableMesh.OnComponentHit`
  (params (HitComponent :type "PrimitiveComponent Object Reference") (OtherActor :type "Actor Object Reference") (OtherComp :type "PrimitiveComponent Object Reference") (NormalImpulse :type "Vector Structure") (Hit :type "HitResult Structure (by ref)"))
  (bind (_bblockinghit _binitialoverlap _time _distance _location) (`GameplayStatics.BreakHitResult` Hit))
  (bind _movablemesh (`self.MovableMesh`))
  (if (`self.CanHit`)
    (if (not (`self.IsDestroyed`))
      (set `self.CanHit` false)
      (if (> (`KismetMathLibrary.VSize` NormalImpulse) 25000000.0)
        (`GameplayStatics.PlaySoundAtLocation` "/Game/StarterContent/Audio/Explosion02.Explosion02" _location (struct) 1.0 1.0 0.0 null null null)
        (if (>= (`self.HitCount`) 10.0)
          (`SceneComponent.SetHiddenInGame` (`self.PhysicsConstraint`) true false)
          (`SceneComponent.SetHiddenInGame` _movablemesh true false)
          (if (not (`self.IsDestroyed`))
            (`GameplayStatics.SpawnEmitterAtLocation` "/Game/StarterContent/Particles/P_Smoke.P_Smoke" (`SceneComponent.K2_GetComponentLocation` _movablemesh))
            (bind _returnvalue (`AddComponent|NODE_AddDestructibleComponent-1`))
            (`DestructibleComponent.SetDestructibleMesh` _returnvalue "/Game/Buildings/BuildingB/BuildingB_Mesh_DM.BuildingB_Mesh_DM")
            (set `self.IsDestroyed` true))
          (else
            (`GameplayStatics.SpawnEmitterAtLocation` "/Game/P_MeshExplosion.P_MeshExplosion" _location)
            (set `self.HitCount` (+ (`self.HitCount`) 1.0))))))))

(fn `UserConstructionScript`)