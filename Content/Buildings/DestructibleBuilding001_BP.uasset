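; Destructible building Blueprint with a physics-constrained movable mesh, meant to collapse after repeated heavy impacts.
; The OnComponentHit event is empty, so the impact and destruction logic is disconnected and never runs; only a timer is set on BeginPlay.
; That orphaned logic filters hits by impulse and cooldown, plays explosion effects, then hides the mesh and spawns a destructible component with smoke once the hit count is reached.
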(event `self.ReceiveBeginPlay`
  (set `self.HitTimer` (`GameplayStatics.GetTimeSeconds`)))

(event `self.MovableMesh.OnComponentHit`
  (params (HitComponent :type "PrimitiveComponent Object Reference") (OtherActor :type "Actor Object Reference") (OtherComp :type "PrimitiveComponent Object Reference") (NormalImpulse :type "Vector Structure") (Hit :type "HitResult Structure (by ref)")))

(fn `UserConstructionScript`)