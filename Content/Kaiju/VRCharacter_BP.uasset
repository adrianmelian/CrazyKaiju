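; VR player character for a Kaiju game that tracks fist input and gives haptic feedback on left-hand contact.
; On begin play it sets the tracking origin to floor level.
; Axis inputs, including the right motion controller trigger, feed separate left and right fist strength variables.
; Overlaps and hits on the left hand hitbox play a medium buzz on the left controller; the right hand has no such handling here.
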(event `self.ReceiveBeginPlay`
  ;[1 1 1] Set Tracking Height
  (`HeadMountedDisplayFunctionLibrary.SetTrackingOrigin` "Floor"))

(event `InputAxis|FistRightFloat`
  (params (AxisValue :type "Float (single-precision)"))
  (set `self.FistRightStrength` (stale `InputAxisKey|MotionController_Right_TriggerAxis` AxisValue) :!label _label))

(event `InputAxisKey|MotionController_Right_TriggerAxis`
  (params (AxisValue :type "Float (single-precision)"))
  (goto _label))

(event `InputAxis|FistLeftFloat`
  (params (AxisValue :type "Float (single-precision)"))
  (set `self.FistLeftStrength` (`self.GetInputAxisKeyValue`)))

(event `self.LeftHand_HitBox.OnComponentBeginOverlap`
  (params (OverlappedComponent :type "PrimitiveComponent Object Reference") (OtherActor :type "Actor Object Reference") (OtherComp :type "PrimitiveComponent Object Reference") (OtherBodyIndex :type Integer) (bFromSweep :type Boolean) (SweepResult :type "HitResult Structure (by ref)"))
  (bind _returnvalue (`MagicLeapControllerFunctionLibrary.GetMotionSourceForHand` "Left" :!label _label_2))
  (`MagicLeapControllerFunctionLibrary.PlayHapticPattern` _returnvalue "Buzz" "Medium"))

(event `self.LeftHand_HitBox.OnComponentHit`
  (params (HitComponent :type "PrimitiveComponent Object Reference") (OtherActor :type "Actor Object Reference") (OtherComp :type "PrimitiveComponent Object Reference") (NormalImpulse :type "Vector Structure") (Hit :type "HitResult Structure (by ref)"))
  (goto _label_2))

(fn `UserConstructionScript`)